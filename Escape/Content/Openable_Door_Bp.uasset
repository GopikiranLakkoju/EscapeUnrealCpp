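; Openable door actor that swings open and closed in response to open and close requests from its OpenDoor source.
; It stores its starting rotation on BeginPlay, then a timeline drives a yaw offset combined with that rotation, so it works at any placed orientation.
; Opening plays the timeline and closing reverses it, with a timeline event track triggering the door sound at the actor's location.
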(event `self.ReceiveBeginPlay`
  ;[1 1 1] Gets initial rotation
  (set `self.Initial Rotation` (`self.K2_GetActorRotation`)))

(event `self.OpenDoor.OnOpenRequest`
  ;[1 1 1] Combines the initial rotation and timeline rotation for relative rotation
  (bind (_direction _door_animation) (`Timeline|Door_Transition` :!label _label)
    (:`Update`
      (`self.K2_SetActorRotation` (`KismetMathLibrary.ComposeRotators` (`KismetMathLibrary.MakeRotator` 0.0 0.0 _door_animation) (`self.Initial Rotation`))))
    (:`Sound Timing`
      (`GameplayStatics.PlaySoundAtLocation` "/Game/Audio/door-close.door-close" (`self.K2_GetActorLocation`) (struct) 1.0 1.0 0.0 null null null))))

(event `self.OpenDoor.OnCloseRequest`
  ;[1 1 1] Combines the initial rotation and timeline rotation for relative rotation
  (goto _label :!via `Reverse`))

(fn `UserConstructionScript`)